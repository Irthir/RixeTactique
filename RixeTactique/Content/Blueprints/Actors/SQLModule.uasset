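; SQLModule is an actor that syncs two-player match state for Rixe Tactique through a remote MySQL database, using hard-coded credentials.
; Once connected, it alternates writing the local player's row and reading the opponent's into Adverse variables, two seconds apart, guarded by RequestOn.
; Change events set the outgoing movement, figurine class codes and victory flag.
; Failed connections retry, but a failed query only prints its error, halting the loop.
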(event `Connect`
  (`self.CreateNewConnection` "aws.connect.psdb.cloud" "rixe_tactique" "sfo1iz73tvfrx47z834f" "pscale_pw_IVaTNGBlg550yY1R0JhF2nh9pBRpkysZomaW1U8USCV" (`|MakeMap` "")))

(event `self.ReceiveBeginPlay`
  (bind _asinstance_rixe (cast `/Game/Blueprints/GameInstance/InstanceRixe` (`GameplayStatics.GetGameInstance`)))
  (set `self.id_unreal` (`/Game/Blueprints/GameInstance/InstanceRixe.idJoueur` _asinstance_rixe))
  (set `self.id_partie` (`/Game/Blueprints/GameInstance/InstanceRixe.idPartie` _asinstance_rixe))
  (if (and (`KismetStringLibrary.NotEqual_StrStr` (`self.id_unreal`)) (`KismetStringLibrary.NotEqual_StrStr` (`self.id_partie`)))
    (`self.Connect`)))

(event `Update`
  ;[1 1 1] Requêtes
  (if (not (`self.bRequestOn`))
    (set `self.bRequestOn` true)
    (`self.UpdateDataFromQuery` (`self.Connection ID`) (`KismetStringLibrary.Concat_StrStr` "UPDATE Joueur \nSET actualisation = CURRENT_TIMESTAMP()," "mouvement = " (`KismetStringLibrary.Conv_IntToString` (`self.nMouvement`)) ", figurine1 = " (`KismetStringLibrary.Conv_IntToString` (`self.Figurine1`)) ", figurine2 = " (`KismetStringLibrary.Conv_IntToString` (`self.Figurine2`)) ", figurine3 = " (`KismetStringLibrary.Conv_IntToString` (`self.Figurine3`)) ", victoire = " (`KismetStringLibrary.Conv_IntToString` (`self.Victoire`)) " WHERE id_unreal = \"" (`self.id_unreal`) "\";"))))

(event `self.ReceiveTick`
  (params (DeltaSeconds :type "Float (single-precision)")))

(event `self.OnConnectionStateChanged`
  (params (ConnectionStatus :type Boolean) (ConnectionID :type Integer) (ErrorMessage :type String))
  (set `self.bRequestOn` false)
  (set `self.Connection ID` ConnectionID)
  (if ConnectionStatus
    (`self.Update`)
    (else
      (`KismetSystemLibrary.PrintString` ErrorMessage)
      (`self.Connect`))))

(event `Select`
  ;[1 1 1] Requêtes
  (if (not (`self.bRequestOn`))
    (set `self.bRequestOn` true)
    (`self.SelectDataFromQuery` (`self.Connection ID`) (`KismetStringLibrary.Concat_StrStr` "SELECT mouvement, figurine1, figurine2, figurine3, victoire \nFROM Joueur \nWHERE partie_id = \"" (`self.id_partie`) "\" AND id_unreal!=\"" (`self.id_unreal`) "\";"))))

(event `self.OnQueryUpdateStatusChanged`
  (params (IsSuccessful :type Boolean) (ErrorMessage :type String))
  (set `self.bRequestOn` false)
  (if IsSuccessful
    (`KismetSystemLibrary.Delay` 2.0)
    (`self.Select`)
    (else
      (`KismetSystemLibrary.PrintString` ErrorMessage))))

(event `self.OnQuerySelectStatusChanged`
  (params (IsSuccessful :type Boolean) (ErrorMessage :type String) (ResultByColumn :type "Array of MySQLDataTable Structure (by ref)") (ResultByRow :type "Array of MySQLDataRow Structure (by ref)"))
  (set `self.bRequestOn` false)
  (if IsSuccessful
    (for _array_element ResultByRow
      (for (_array_element_2 _array_index) (break `MySQLDataRow` _array_element)
        (switch `int` _array_index
          (:`0`
            (bind _returnvalue (`KismetStringLibrary.Conv_StringToInt` _array_element_2))
            (set `self.adverseMouvement` _returnvalue))
          (:`1`
            (set `self.adverseFigurine1` _returnvalue))
          (:`2`
            (set `self.adverseFigurine2` _returnvalue))
          (:`3`
            (set `self.adverseFigurine3` _returnvalue))
          (:`4`
            (set `self.adverseVictoire` _returnvalue)))))
    (`KismetSystemLibrary.Delay` 2.0)
    (`self.Update`)
    (else
      (`KismetSystemLibrary.PrintString` ErrorMessage))))

(event `ChangeVictoire`
  (params (bVictoire :type Boolean))
  (if bVictoire
    (set `self.Victoire` 1)
    (else
      (set `self.Victoire` -1))))

(event `ChangeMouvement`
  (params (nMouvement :type Integer))
  (set `self.nMouvement` nMouvement))

(event `ChangeFigurine`
  (params (Figurine1 :type "EFigurine Enum" :default "Guerrier") (Figurine2 :type "EFigurine Enum" :default "Guerrier") (Figurine3 :type "EFigurine Enum" :default "Guerrier"))
  (switch `EFigurine` Figurine1
    (:`Guerrier`
      (set `self.Figurine1` 1))
    (:`Mage`
      (set `self.Figurine1` 2))
    (:`Voleur`
      (set `self.Figurine1` 3))
    (:`Eclaireur`
      (set `self.Figurine1` 4))
    (:`Pretre`
      (set `self.Figurine1` 5))
    (:`Protecteur`
      (set `self.Figurine1` 6)))
  (switch `EFigurine` Figurine2
    (:`Guerrier`
      (set `self.Figurine2` 1))
    (:`Mage`
      (set `self.Figurine2` 2))
    (:`Voleur`
      (set `self.Figurine2` 3))
    (:`Eclaireur`
      (set `self.Figurine2` 4))
    (:`Pretre`
      (set `self.Figurine2` 5))
    (:`Protecteur`
      (set `self.Figurine2` 6)))
  (switch `EFigurine` Figurine3
    (:`Guerrier`
      (set `self.Figurine3` 1))
    (:`Mage`
      (set `self.Figurine3` 2))
    (:`Voleur`
      (set `self.Figurine3` 3))
    (:`Eclaireur`
      (set `self.Figurine3` 4))
    (:`Pretre`
      (set `self.Figurine3` 5))
    (:`Protecteur`
      (set `self.Figurine3` 6))))

(fn `UserConstructionScript`)