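; SQLMenu is the matchmaking lobby actor for hosting, listing and joining two-player games through a remote SQL database, using hardcoded credentials.
; Query callbacks and boolean flags chain timestamp-keyed Joueur and Partie inserts, then heartbeat-poll until the host gets an opponent.
; Search feeds recently active one-player games to the menu widget.
; Successful pairing calls InstanceRixe.Lancement, while SQL errors restart the game.
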(event `Lancement`
  (params (idJoueur :type String) (idPartie :type String))
  (bind _asinstance_rixe (cast `/Game/Blueprints/GameInstance/InstanceRixe` (`GameplayStatics.GetGameInstance`)))
  (`/Game/Blueprints/GameInstance/InstanceRixe.Lancement` _asinstance_rixe idJoueur idPartie))

(event `self.ReceiveBeginPlay`
  (`self.CreateNewConnection` "aws.connect.psdb.cloud" "rixe_tactique" "sfo1iz73tvfrx47z834f" "pscale_pw_IVaTNGBlg550yY1R0JhF2nh9pBRpkysZomaW1U8USCV" (`|MakeMap` "")))

(event `CreationJoueur`
  ;[1 1 1] Creation Joueur
  (`self.UpdateDataFromQuery` (`self.Connection ID`) (`KismetStringLibrary.Concat_StrStr` "INSERT INTO Joueur \n(id_unreal, actualisation, partie_id, name) \nVALUES \n(\"" (`self.id_unreal`) "\", CURRENT_TIMESTAMP(), \"" (`self.id_partie`) "\",\"" (`KismetSystemLibrary.GetPlatformUserName`) "\");")))

(event `UpdateJoueur`
  ;[1 1 1] MàJ Joueur
  (`self.UpdateDataFromQuery` (`self.Connection ID`) (`KismetStringLibrary.Concat_StrStr` "UPDATE Joueur \nSET actualisation = CURRENT_TIMESTAMP() \nWHERE id_unreal = \"" (`self.id_unreal`) "\";")))

(event `self.ReceiveTick`
  (params (DeltaSeconds :type "Float (single-precision)")))

(event `JoinPartie`
  ;[1 1 1] RejoindrePartie
  (`self.UpdateDataFromQuery` (`self.Connection ID`) (`KismetStringLibrary.Concat_StrStr` "UPDATE Joueur \nSET actualisation = CURRENT_TIMESTAMP(), \npartie_id = \"" (`self.id_partie`) "\" \nWHERE id_unreal = \"" (`self.id_unreal`) "\";")))

(event `self.OnConnectionStateChanged`
  (params (ConnectionStatus :type Boolean) (ConnectionID :type Integer) (ErrorMessage :type String))
  (bind (_returnvalue_year _returnvalue_month _returnvalue_day _returnvalue_hour _returnvalue_minute _returnvalue_second _returnvalue_millisecond) (`KismetMathLibrary.BreakDateTime` (`KismetMathLibrary.Now`)))
  (if ConnectionStatus
    (set `self.Connection ID` ConnectionID)
    (set `self.id_unreal` (`KismetStringLibrary.Concat_StrStr` (`KismetStringLibrary.Conv_IntToString` _returnvalue_year) (`KismetStringLibrary.Conv_IntToString` _returnvalue_month) (`KismetStringLibrary.Conv_IntToString` _returnvalue_day) (`KismetStringLibrary.Conv_IntToString` _returnvalue_hour) (`KismetStringLibrary.Conv_IntToString` _returnvalue_minute) (`KismetStringLibrary.Conv_IntToString` _returnvalue_second) (`KismetStringLibrary.Conv_IntToString` _returnvalue_millisecond)))
    (else
      (`KismetSystemLibrary.PrintString` ErrorMessage)
      (`self.Reset`))))

(event `Host`
  (params (NomPartie :type String))
  (bind (_returnvalue_year _returnvalue_month _returnvalue_day _returnvalue_hour _returnvalue_minute _returnvalue_second _returnvalue_millisecond) (`KismetMathLibrary.BreakDateTime` (`KismetMathLibrary.Now`)))
  (if (not (or (`self.bAttenteJoueur`) (`self.bCreationJoin`) (`self.bCreationHost`)))
    (set `self.bCreationHost` true)
    (set `self.Nom Partie` NomPartie)
    (set `self.id_partie` (`KismetStringLibrary.Concat_StrStr` (`KismetStringLibrary.Conv_IntToString` _returnvalue_year) (`KismetStringLibrary.Conv_IntToString` _returnvalue_month) (`KismetStringLibrary.Conv_IntToString` _returnvalue_day) (`KismetStringLibrary.Conv_IntToString` _returnvalue_hour) (`KismetStringLibrary.Conv_IntToString` _returnvalue_minute) (`KismetStringLibrary.Conv_IntToString` _returnvalue_second) (`KismetStringLibrary.Conv_IntToString` _returnvalue_millisecond)))
    (`self.CreationJoueur`)))

(event `CreationPartie`
  ;[1 1 1] CreationPartie
  (`self.UpdateDataFromQuery` (`self.Connection ID`) (`KismetStringLibrary.Concat_StrStr` "INSERT INTO Partie \n(id_unreal, nom) \nVALUES \n(\"" (`self.id_partie`) "\", \"" (`self.Nom Partie`) "\");")))

(event `Join`
  (params (id_partie :type String))
  (if (not (or (`self.bAttenteJoueur`) (`self.bCreationJoin`) (`self.bCreationHost`)))
    (set `self.bCreationJoin` true)
    (set `self.id_partie` id_partie)
    (`self.CreationJoueur`)))

(event `SelectSelf`
  (`self.SelectDataFromQuery` (`self.Connection ID`) (`KismetStringLibrary.Concat_StrStr` "SELECT * \nFROM Joueur \nWHERE id_unreal = \"" (`self.id_unreal`) "\";")))

(event `self.OnQueryUpdateStatusChanged`
  (params (IsSuccessful :type Boolean) (ErrorMessage :type String))
  (if IsSuccessful
    (if (`self.bRejoindrePartie`)
      (`KismetSystemLibrary.PrintString` (`KismetStringLibrary.Concat_StrStr` "Partie rejointe : " (`self.Nom Partie`)))
      (`self.Lancement` (`self.id_unreal`) (`self.id_partie`))
      (elif (`self.bUpdate`)
        (set `self.bUpdate` false)
        (`self.SelectNbJoueurPartie`)
        (elif (`self.bCreationHost`)
          (if (`self.bPartieCree`)
            (`self.SelectNbJoueurPartie`)
            (else
              (`self.CreationPartie`)
              (set `self.bPartieCree` true)))
          (elif (`self.bCreationJoin`)
            (set `self.bCreationJoin` false)))))
    (else
      (`KismetSystemLibrary.PrintString` ErrorMessage)
      (`self.Reset`))))

(event `SelectAdverse`
  (`self.SelectDataFromQuery` (`self.Connection ID`) (`KismetStringLibrary.Concat_StrStr` "SELECT * \nFROM Joueur \nWHERE id_unreal = \"" (`self.id_unreal`) "\";")))

(event `SelectNbJoueurPartie`
  ;[1 1 1] Comment
  (if (not (`self.bAttenteJoueur`))
    (`self.SelectDataFromQuery` (`self.Connection ID`) (`KismetStringLibrary.Concat_StrStr` "SELECT * \nFROM Joueur \nWHERE partie_id = \"" (`self.id_partie`) "\";"))
    (set `self.bAttenteJoueur` true)))

(event `SelectPartie`
  (`self.SelectDataFromQuery` (`self.Connection ID`) (`KismetStringLibrary.Concat_StrStr` "SELECT id_unreal, nom \nFROM Partie \nWHERE id_unreal IN( \n	SELECT partie_id \n	FROM Joueur \n	WHERE TIMESTAMPDIFF(MINUTE,actualisation, CURRENT_TIMESTAMP())<=5  \n	AND partie_id NOT IN ( \n		SELECT partie_id as pid \n		FROM Joueur \n		GROUP BY pid \n		HAVING COUNT(pid) >1) \n	);")))

(event `self.OnQuerySelectStatusChanged`
  (params (IsSuccessful :type Boolean) (ErrorMessage :type String) (ResultByColumn :type "Array of MySQLDataTable Structure (by ref)") (ResultByRow :type "Array of MySQLDataRow Structure (by ref)"))
  (bind _interfacemenu (`self.InterfaceMenu`))
  (if IsSuccessful
    (if (`self.bRecherchePartie`)
      (set `self.bRecherchePartie` false)
      (`/Engine/EditorBlueprintResources/StandardMacros.IsValid` _interfacemenu
        (:`Is Valid`
          (`/Game/Blueprints/Widgets/InterfaceMenuPrincipal.ResetAffichePartie` _interfacemenu)
          (for _array_element ResultByRow
            (if (and (`KismetStringLibrary.NotEqual_StrStr` (`|GetArrayItem` (break `MySQLDataRow` _array_element))) (`KismetStringLibrary.NotEqual_StrStr` (`|GetArrayItem` (break `MySQLDataRow` _array_element) 1)))
              (`/Game/Blueprints/Widgets/InterfaceMenuPrincipal.AddPartie` _interfacemenu (break `MySQLDataRow` _array_element))))))
      (elif (`self.bAttenteJoueur`)
        (set `self.bAttenteJoueur` false)
        (if (> (`KismetArrayLibrary.Array_Length` ResultByRow) 1)
          (`KismetSystemLibrary.PrintString` "Connexion d'un client !")
          (set `self.bCreationHost` false)
          (`self.Lancement` (`self.id_unreal`) (`self.id_partie`))
          (else
            (`KismetSystemLibrary.Delay` 2.0)
            (set `self.bUpdate` true)
            (`self.UpdateJoueur`)
            (`KismetSystemLibrary.PrintString` "Attente d'un client.")))))
    (else
      (`KismetSystemLibrary.PrintString` ErrorMessage)
      (`self.Reset`))))

(event `RecherchePartie`
  (params (InterfaceMenu :type "/Game/Blueprints/Widgets/InterfaceMenuPrincipal Object Reference"))
  ;[1 1 1] Comment
  (set `self.InterfaceMenu` InterfaceMenu)
  (if (not (`self.bRecherchePartie`))
    (set `self.bRecherchePartie` true)
    (`self.SelectDataFromQuery` (`self.Connection ID`) (`KismetStringLibrary.Concat_StrStr` "SELECT id_unreal, nom \nFROM Partie \nWHERE id_unreal IN( \n	SELECT partie_id \n	FROM Joueur \n	WHERE TIMESTAMPDIFF(MINUTE,actualisation, CURRENT_TIMESTAMP())<=5  \n	AND partie_id IN ( \n		SELECT partie_id \n		FROM Joueur \n		GROUP BY partie_id \n		HAVING COUNT(partie_id) =1) \n	);"))))

(event `RejoindrePartie`
  (params (NomPartie :type String) (IdPartie :type String))
  (set `self.id_partie` IdPartie)
  (set `self.Nom Partie` NomPartie)
  (set `self.bRejoindrePartie` true)
  (`self.Join` (`self.id_partie`)))

(event `self.ReceiveDestroyed`)

(event `Reset`
  (bind _asgame_mode (cast `GameMode` (`GameplayStatics.GetGameMode`)))
  (`GameMode.RestartGame` _asgame_mode))

(fn `UserConstructionScript`)