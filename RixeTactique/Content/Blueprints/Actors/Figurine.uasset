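; Figurine actor that glides toward a target location stored in a variable.
; BeginPlay sets both the target and the saved position to the actor's starting location.
; Each Tick moves the actor toward the target by a lerp with DeltaSeconds as alpha, giving an eased approach without sweep.
; The saved position updates only once the location exactly matches the target; nothing in this file changes the target after BeginPlay.
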(event `self.ReceiveBeginPlay`
  (bind _returnvalue (`self.K2_GetActorLocation`))
  (set `self.vTarget` _returnvalue)
  (set `self.vPosition` _returnvalue))

(event `self.ReceiveTick`
  (params (DeltaSeconds :type "Float (single-precision)"))
  (if (!= (`self.vTarget`) (`self.K2_GetActorLocation`))
    (`self.K2_SetActorLocation` self (`KismetMathLibrary.VLerp` (`self.K2_GetActorLocation` self) (`self.vTarget`) DeltaSeconds) false false)
    (else
      (set `self.vPosition` (`self.K2_GetActorLocation`)))))

(fn `UserConstructionScript`)