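; DonjonManager actor that builds the dungeon as a square grid of DonjonSalle rooms centred around itself and starts the players in it.
; Tick gathers Player actors, then spawns the rooms once and links their north, south, east and west neighbours by array index.
; Each SchemaMap DataTable row configures the room at the same index.
; TestVisibility then has every room check visibility and player distance.
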(event `self.ReceiveTick`
  (params (DeltaSeconds :type "Float (single-precision)"))
  (bind (_returnvalue_x _returnvalue_y _returnvalue_z) (`KismetMathLibrary.BreakVector` (`self.K2_GetActorLocation` self)))
  (bind _returnvalue (/ (`self.nTailleDonjon`) 2))
  (bind _returnvalue_2 (* _returnvalue -1))
  (if (`KismetSystemLibrary.IsServer`)
    _
    (else
      _))
  (`/Engine/EditorBlueprintResources/StandardMacros.IsValid` (`|GetArrayItem` (`self.Players`))
    (:`Is Valid`
      _)
    (:`Is Not Valid`
      (bind _outactors (`GameplayStatics.GetAllActorsOfClass` "/Game/Blueprints/Pawns/Player.Player_C"))
      (bind _output_get (set `self.Players` _outactors))))
  (if (>= (`KismetArrayLibrary.Array_Length` _output_get) 1)
    ;[1 0 0.07563] Apparition des salles du donjon
    (`/Engine/EditorBlueprintResources/StandardMacros.DoOnce` false
      (:`Completed`
        (for _index (range _returnvalue_2 (+ _returnvalue 1))
          (for _index_2 (range _returnvalue_2 (+ _returnvalue 1))
            (bind _returnvalue_3 (`|SpawnActorFromClass` "/Game/Blueprints/Actors/DonjonSalle.DonjonSalle_C" (`KismetMathLibrary.MakeTransform` (`KismetMathLibrary.MakeVector` (* (+ _returnvalue_x (* (`self.fDistanceSalle`) _index)) -1.0) (+ _returnvalue_y (* (`self.fDistanceSalle`) _index_2)) _returnvalue_z)) "AlwaysSpawn" "OverrideRootScale" null null))
            ;;[1 1 1] Initialisation des données des salles
            (set `/Game/Blueprints/Actors/DonjonSalle.yIndex` _index_2 _returnvalue_3)
            (set `/Game/Blueprints/Actors/DonjonSalle.xIndex` _index _returnvalue_3)
            (set `/Game/Blueprints/Actors/DonjonSalle.DonjonManager` self _returnvalue_3)
            (`/Game/Blueprints/Actors/DonjonSalle.Initialisation` _returnvalue_3)
            (`KismetArrayLibrary.Array_Add` (`self.tSalles`) _returnvalue_3)))
        (`self.SetSallesCardinaux`)
        (`self.GenerationDonjon`)))))

(event `SetSallesCardinaux`
  ;[1 1 1] Mise en place des cardinaux des salles
  (for (_array_element _array_index) (`self.tSalles`)
    (bind _returnvalue (- _array_index (`self.nTailleDonjon`)))
    (if (>= _returnvalue 0)
      (`/Game/Blueprints/Actors/DonjonSalle.AddNord` _array_element (`|GetArrayItem` (`self.tSalles`) _returnvalue)))
    (bind _returnvalue_2 (+ _array_index (`self.nTailleDonjon`)))
    (if (< _returnvalue_2 (`KismetArrayLibrary.Array_Length` (`self.tSalles`)))
      (`/Game/Blueprints/Actors/DonjonSalle.AddSud` _array_element (`|GetArrayItem` (`self.tSalles`) _returnvalue_2)))
    (bind _returnvalue_3 (+ _array_index 1))
    (if (!= (mod _returnvalue_3 (`self.nTailleDonjon`)) 0)
      (`/Game/Blueprints/Actors/DonjonSalle.AddEst` _array_element (`|GetArrayItem` (`self.tSalles`) _returnvalue_3)))
    (bind _returnvalue_4 (- _array_index 1))
    (if (and (>= _returnvalue_4 0) (!= (mod _array_index (`self.nTailleDonjon`)) 0))
      (`/Game/Blueprints/Actors/DonjonSalle.AddOuest` _array_element (`|GetArrayItem` (`self.tSalles`) _returnvalue_4)))))

(event `GenerationDonjon`
  (bind _returnvalue (`DataTableFunctionLibrary.GetDataTableColumnAsString` "/Game/Data/SchemaMap.SchemaMap" "tElementSalle"))
  (for (_array_element _array_index) _returnvalue
    (`/Game/Blueprints/Actors/DonjonSalle.SetSalleInfo` (`|GetArrayItem` (`self.tSalles`) _array_index) _array_element))
  (for _array_element_2 (`self.Players`)
    (`/Game/Blueprints/Pawns/Player.Start` _array_element_2))
  (`self.TestVisibility`))

(event `TestVisibility`
  (for _array_element (`self.tSalles`)
    (`/Game/Blueprints/Actors/DonjonSalle.TestVisibility` _array_element)
    (`/Game/Blueprints/Actors/DonjonSalle.CheckDistanceJoueur` _array_element)))

(fn `UserConstructionScript`)