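; NetWorkObject is an actor that appears meant as a single network helper in the level.
; On BeginPlay it finds all NetWorkObject actors and destroys itself if more than one exists.
; Its ValideClient event takes a Valide input but only branches on IsServer, with nothing attached.
; Unconnected debug nodes would print each Player's NbMouvement and a client/server string, while Tick and construction are empty.
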(event `self.ReceiveBeginPlay`
  (bind _outactors (`GameplayStatics.GetAllActorsOfClass` "NetWorkObject_C"))
  (if (> (`KismetArrayLibrary.Array_Length` _outactors) 1)
    (`self.K2_DestroyActor`)))

(event `self.ReceiveTick`
  (params (DeltaSeconds :type "Float (single-precision)")))

(event `ValideClient`
  (params (Valide :type Boolean))
  (if (`KismetSystemLibrary.IsServer`)
    _))

(fn `UserConstructionScript`)