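; Dungeon room actor for a grid dungeon, linked to its four neighbours.
; Initialisation strips duplicate walls and pillars off non-edge rooms, so wall and door calls or queries forward to the neighbour owning the shared wall.
; SetSalleInfo turns a data string into doorways and a room event, with some random rolls, and places player one on J1.
; It also drives minimap sprites and icons by discovery state and hides geometry far from the player.
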(event `CheckDistanceJoueur`
  (bind _pilliersudouest (`self.pillierSudOuest`))
  (bind _pilliernordest (`self.pillierNordEst`))
  (bind _pilliernordouest (`self.pillierNordOuest`))
  (bind _pilliersudest (`self.pillierSudEst`))
  (bind _murest (`self.murEst`))
  (bind _murnord (`self.murNord`))
  (bind _mursud (`self.murSud`))
  (bind _murouest (`self.murOuest`))
  (bind _pilliersudouest_2 (`self.pillierSudOuest`))
  (bind _pilliernordest_2 (`self.pillierNordEst`))
  (bind _pilliernordouest_2 (`self.pillierNordOuest`))
  (bind _pilliersudest_2 (`self.pillierSudEst`))
  (bind _murest_2 (`self.murEst`))
  (bind _murnord_2 (`self.murNord`))
  (bind _mursud_2 (`self.murSud`))
  (bind _murouest_2 (`self.murOuest`))
  (bind _sol (`self.sol`))
  (bind _sol_2 (`self.sol`))
  (bind _returnvalue_location (`KismetMathLibrary.BreakTransform` (`self.GetTransform` self)))
  (bind _returnvalue_location_2 (`KismetMathLibrary.BreakTransform` (`self.GetTransform` (`GameplayStatics.GetPlayerPawn` 0))))
  (if (> (`KismetMathLibrary.Vector_Distance` _returnvalue_location _returnvalue_location_2) 2500.0)
    (`/Engine/EditorBlueprintResources/StandardMacros.IsValid` _pilliersudouest_2
      (:`Is Valid`
        (`SceneComponent.SetHiddenInGame` _pilliersudouest_2 true false))
      (:`Is Not Valid`
        _))
    (`/Engine/EditorBlueprintResources/StandardMacros.IsValid` _pilliernordest_2
      (:`Is Valid`
        (`SceneComponent.SetHiddenInGame` _pilliernordest_2 true false))
      (:`Is Not Valid`
        _))
    (`/Engine/EditorBlueprintResources/StandardMacros.IsValid` _pilliernordouest_2
      (:`Is Valid`
        (`SceneComponent.SetHiddenInGame` _pilliernordouest_2 true false))
      (:`Is Not Valid`
        _))
    (`/Engine/EditorBlueprintResources/StandardMacros.IsValid` _pilliersudest_2
      (:`Is Valid`
        (`SceneComponent.SetHiddenInGame` _pilliersudest_2 true false))
      (:`Is Not Valid`
        _))
    (`/Engine/EditorBlueprintResources/StandardMacros.IsValid` _murest_2
      (:`Is Valid`
        (`SceneComponent.SetHiddenInGame` _murest_2 true false))
      (:`Is Not Valid`
        _))
    (`/Engine/EditorBlueprintResources/StandardMacros.IsValid` _murnord_2
      (:`Is Valid`
        (`SceneComponent.SetHiddenInGame` _murnord_2 true false))
      (:`Is Not Valid`
        _))
    (`/Engine/EditorBlueprintResources/StandardMacros.IsValid` _mursud_2
      (:`Is Valid`
        (`SceneComponent.SetHiddenInGame` _mursud_2 true false))
      (:`Is Not Valid`
        _))
    (`/Engine/EditorBlueprintResources/StandardMacros.IsValid` _murouest_2
      (:`Is Valid`
        (`SceneComponent.SetHiddenInGame` _murouest_2 true false))
      (:`Is Not Valid`
        _))
    (`/Engine/EditorBlueprintResources/StandardMacros.IsValid` _sol_2
      (:`Is Valid`
        (`SceneComponent.SetHiddenInGame` _sol_2 true false)))
    (else
      (`/Engine/EditorBlueprintResources/StandardMacros.IsValid` _pilliersudouest
        (:`Is Valid`
          (`SceneComponent.SetHiddenInGame` _pilliersudouest false false))
        (:`Is Not Valid`
          _))
      (`/Engine/EditorBlueprintResources/StandardMacros.IsValid` _pilliernordest
        (:`Is Valid`
          (`SceneComponent.SetHiddenInGame` _pilliernordest false false))
        (:`Is Not Valid`
          _))
      (`/Engine/EditorBlueprintResources/StandardMacros.IsValid` _pilliernordouest
        (:`Is Valid`
          (`SceneComponent.SetHiddenInGame` _pilliernordouest false false))
        (:`Is Not Valid`
          _))
      (`/Engine/EditorBlueprintResources/StandardMacros.IsValid` _pilliersudest
        (:`Is Valid`
          (`SceneComponent.SetHiddenInGame` _pilliersudest false false))
        (:`Is Not Valid`
          _))
      (`/Engine/EditorBlueprintResources/StandardMacros.IsValid` _murest
        (:`Is Valid`
          (`SceneComponent.SetHiddenInGame` _murest false false))
        (:`Is Not Valid`
          _))
      (`/Engine/EditorBlueprintResources/StandardMacros.IsValid` _murnord
        (:`Is Valid`
          (`SceneComponent.SetHiddenInGame` _murnord false false))
        (:`Is Not Valid`
          _))
      (`/Engine/EditorBlueprintResources/StandardMacros.IsValid` _mursud
        (:`Is Valid`
          (`SceneComponent.SetHiddenInGame` _mursud false false))
        (:`Is Not Valid`
          _))
      (`/Engine/EditorBlueprintResources/StandardMacros.IsValid` _murouest
        (:`Is Valid`
          (`SceneComponent.SetHiddenInGame` _murouest false false))
        (:`Is Not Valid`
          _))
      (`/Engine/EditorBlueprintResources/StandardMacros.IsValid` _sol
        (:`Is Valid`
          (`SceneComponent.SetHiddenInGame` _sol false false))))))

(event `HideMiniMap`
  (bind _paperspritenordouest (`self.PaperSpriteNordOuest`))
  (bind _paperspritesudest (`self.PaperSpriteSudEst`))
  (bind _paperspriteest (`self.PaperSpriteEst`))
  (bind _paperspritenordest (`self.PaperSpriteNordEst`))
  (bind _paperspritenord (`self.PaperSpriteNord`))
  (bind _paperspritesudouest (`self.PaperSpriteSudOuest`))
  (bind _paperspritesud (`self.PaperSpriteSud`))
  (bind _paperspriteouest (`self.PaperSpriteOuest`))
  (`/Engine/EditorBlueprintResources/StandardMacros.IsValid` _paperspritenordouest
    (:`Is Valid`
      (`SceneComponent.SetVisibility` _paperspritenordouest false false))
    (:`Is Not Valid`
      _))
  (`/Engine/EditorBlueprintResources/StandardMacros.IsValid` _paperspriteouest
    (:`Is Valid`
      (`SceneComponent.SetVisibility` _paperspriteouest false false))
    (:`Is Not Valid`
      _))
  (`/Engine/EditorBlueprintResources/StandardMacros.IsValid` _paperspritesud
    (:`Is Valid`
      (`SceneComponent.SetVisibility` _paperspritesud false false))
    (:`Is Not Valid`
      _))
  (`/Engine/EditorBlueprintResources/StandardMacros.IsValid` _paperspritesudouest
    (:`Is Valid`
      (`SceneComponent.SetVisibility` _paperspritesudouest false false))
    (:`Is Not Valid`
      _))
  (`/Engine/EditorBlueprintResources/StandardMacros.IsValid` _paperspritenord
    (:`Is Valid`
      (`SceneComponent.SetVisibility` _paperspritenord false false))
    (:`Is Not Valid`
      _))
  (`/Engine/EditorBlueprintResources/StandardMacros.IsValid` _paperspritenordest
    (:`Is Valid`
      (`SceneComponent.SetVisibility` _paperspritenordest false false))
    (:`Is Not Valid`
      _))
  (`/Engine/EditorBlueprintResources/StandardMacros.IsValid` _paperspriteest
    (:`Is Valid`
      (`SceneComponent.SetVisibility` _paperspriteest false false))
    (:`Is Not Valid`
      _))
  (`/Engine/EditorBlueprintResources/StandardMacros.IsValid` _paperspritesudest
    (:`Is Valid`
      (`SceneComponent.SetVisibility` _paperspritesudest false false)
      (`SceneComponent.SetVisibility` (`self.PaperSpriteIcone`) false false))))

(event `ShowMiniMap`
  (bind _paperspritenordouest (`self.PaperSpriteNordOuest`))
  (bind _paperspritesudest (`self.PaperSpriteSudEst`))
  (bind _paperspriteest (`self.PaperSpriteEst`))
  (bind _paperspritenordest (`self.PaperSpriteNordEst`))
  (bind _paperspritenord (`self.PaperSpriteNord`))
  (bind _paperspritesudouest (`self.PaperSpriteSudOuest`))
  (bind _paperspritesud (`self.PaperSpriteSud`))
  (bind _paperspriteouest (`self.PaperSpriteOuest`))
  (`/Engine/EditorBlueprintResources/StandardMacros.IsValid` _paperspritenordouest
    (:`Is Valid`
      (`SceneComponent.SetVisibility` _paperspritenordouest true false))
    (:`Is Not Valid`
      _))
  (`/Engine/EditorBlueprintResources/StandardMacros.IsValid` _paperspriteouest
    (:`Is Valid`
      (`SceneComponent.SetVisibility` _paperspriteouest true false))
    (:`Is Not Valid`
      _))
  (`/Engine/EditorBlueprintResources/StandardMacros.IsValid` _paperspritesud
    (:`Is Valid`
      (`SceneComponent.SetVisibility` _paperspritesud true false))
    (:`Is Not Valid`
      _))
  (`/Engine/EditorBlueprintResources/StandardMacros.IsValid` _paperspritesudouest
    (:`Is Valid`
      (`SceneComponent.SetVisibility` _paperspritesudouest true false))
    (:`Is Not Valid`
      _))
  (`/Engine/EditorBlueprintResources/StandardMacros.IsValid` _paperspritenord
    (:`Is Valid`
      (`SceneComponent.SetVisibility` _paperspritenord true false))
    (:`Is Not Valid`
      _))
  (`/Engine/EditorBlueprintResources/StandardMacros.IsValid` _paperspritenordest
    (:`Is Valid`
      (`SceneComponent.SetVisibility` _paperspritenordest true false))
    (:`Is Not Valid`
      _))
  (`/Engine/EditorBlueprintResources/StandardMacros.IsValid` _paperspriteest
    (:`Is Valid`
      (`SceneComponent.SetVisibility` _paperspriteest true false))
    (:`Is Not Valid`
      _))
  (`/Engine/EditorBlueprintResources/StandardMacros.IsValid` _paperspritesudest
    (:`Is Valid`
      (`SceneComponent.SetVisibility` _paperspritesudest true false)
      (`SceneComponent.SetVisibility` (`self.PaperSpriteIcone`) true false))))

(event `self.ReceiveBeginPlay`
  (if (not (`self.ConnueJ1`))
    (`self.HideMiniMap`)))

(event `TestVisibility`
  (if (`self.ConnueJ1`)
    (`self.ShowMiniMap` :!label _label)
    (elif (`self.VueJ1`)
      (goto _label)
      (else
        (`self.HideMiniMap`))))
  (`self.MasqueMiniCarte`)
  (`self.ChangeIconeSalle`))

(event `Initialisation`
  (set `self.nTailleDonjon` (`/Game/Blueprints/Actors/DonjonManager.nTailleDonjon` (`self.DonjonManager`)))
  (`self.Délétion murs et piliers`))

(event `AddNord`
  (params (Salle :type "/Game/Blueprints/Actors/DonjonSalle Object Reference"))
  (set `self.SalleNord` Salle))

(event `AddSud`
  (params (Salle :type "/Game/Blueprints/Actors/DonjonSalle Object Reference"))
  (set `self.SalleSud` Salle))

(event `AddEst`
  (params (Salle :type "/Game/Blueprints/Actors/DonjonSalle Object Reference"))
  (set `self.SalleEst` Salle))

(event `AddOuest`
  (params (Salle :type "/Game/Blueprints/Actors/DonjonSalle Object Reference"))
  (set `self.SalleOuest` Salle))

(event `AjoutMurNord`
  (bind _sallenord (`self.SalleNord`))
  (bind _murnord (`self.murNord`))
  (`/Engine/EditorBlueprintResources/StandardMacros.IsValid` _murnord
    (:`Is Valid`
      (`StaticMeshComponent.SetStaticMesh` _murnord "/Game/MedievalDungeon/Meshes/Architecture/Dungeon/SM_Dungeon_Wall.SM_Dungeon_Wall")
      (`SceneComponent.K2_SetRelativeLocation` _murnord (600.0 0.0 0.0) false true))
    (:`Is Not Valid`
      (`/Engine/EditorBlueprintResources/StandardMacros.IsValid` _sallenord
        (:`Is Valid`
          (`self.AjoutMurSud` _sallenord))))))

(event `AjoutPorteNord`
  (bind _murnord (`self.murNord`))
  (bind _sallenord (`self.SalleNord`))
  (`/Engine/EditorBlueprintResources/StandardMacros.IsValid` _murnord
    (:`Is Valid`
      (`StaticMeshComponent.SetStaticMesh` _murnord "/Game/MedievalDungeon/Meshes/Architecture/Dungeon/SM_DoorWay.SM_DoorWay")
      (`SceneComponent.K2_SetRelativeLocation` _murnord (600.0 300.0 0.0) false true))
    (:`Is Not Valid`
      (`/Engine/EditorBlueprintResources/StandardMacros.IsValid` _sallenord
        (:`Is Valid`
          (`self.AjoutPorteSud` _sallenord))
        (:`Is Not Valid`
          (`KismetSystemLibrary.PrintString` "Hello"))))))

(event `AjoutMurEst`
  (bind _murest (`self.murEst`))
  (bind _salleest (`self.SalleEst`))
  (`/Engine/EditorBlueprintResources/StandardMacros.IsValid` _murest
    (:`Is Valid`
      (`StaticMeshComponent.SetStaticMesh` _murest "/Game/MedievalDungeon/Meshes/Architecture/Dungeon/SM_Dungeon_Wall.SM_Dungeon_Wall")
      (`SceneComponent.K2_SetRelativeLocation` _murest (600.0 600.0 0.0) false true))
    (:`Is Not Valid`
      (`/Engine/EditorBlueprintResources/StandardMacros.IsValid` _salleest
        (:`Is Valid`
          (`self.AjoutMurOuest` _salleest))))))

(event `AjoutPorteEst`
  (bind _murest (`self.murEst`))
  (bind _salleest (`self.SalleEst`))
  (`/Engine/EditorBlueprintResources/StandardMacros.IsValid` _murest
    (:`Is Valid`
      (`StaticMeshComponent.SetStaticMesh` _murest "/Game/MedievalDungeon/Meshes/Architecture/Dungeon/SM_DoorWay.SM_DoorWay")
      (`SceneComponent.K2_SetRelativeLocation` _murest (300.0 600.0 0.0) false true))
    (:`Is Not Valid`
      (`/Engine/EditorBlueprintResources/StandardMacros.IsValid` _salleest
        (:`Is Valid`
          (`self.AjoutPorteOuest` _salleest))
        (:`Is Not Valid`
          (`KismetSystemLibrary.PrintString` "Hello"))))))

(event `AjoutMurSud`
  (bind _mursud (`self.murSud`))
  (bind _sallesud (`self.SalleSud`))
  (`/Engine/EditorBlueprintResources/StandardMacros.IsValid` _mursud
    (:`Is Valid`
      (`StaticMeshComponent.SetStaticMesh` _mursud "/Game/MedievalDungeon/Meshes/Architecture/Dungeon/SM_Dungeon_Wall.SM_Dungeon_Wall")
      (`SceneComponent.K2_SetRelativeLocation` _mursud (0.0 0.0 0.0) false true))
    (:`Is Not Valid`
      (`/Engine/EditorBlueprintResources/StandardMacros.IsValid` _sallesud
        (:`Is Valid`
          (`self.AjoutMurNord` _sallesud))))))

(event `AjoutPorteSud`
  (bind _mursud (`self.murSud`))
  (bind _sallesud (`self.SalleSud`))
  (`/Engine/EditorBlueprintResources/StandardMacros.IsValid` _mursud
    (:`Is Valid`
      (`StaticMeshComponent.SetStaticMesh` _mursud "/Game/MedievalDungeon/Meshes/Architecture/Dungeon/SM_DoorWay.SM_DoorWay")
      (`SceneComponent.K2_SetRelativeLocation` _mursud (0.0 300.0 0.0) false true))
    (:`Is Not Valid`
      (`/Engine/EditorBlueprintResources/StandardMacros.IsValid` _sallesud
        (:`Is Valid`
          (`self.AjoutPorteNord` _sallesud))
        (:`Is Not Valid`
          (`KismetSystemLibrary.PrintString` "Hello"))))))

(event `AjoutMurOuest`
  (bind _murouest (`self.murOuest`))
  (bind _salleouest (`self.SalleOuest`))
  (`/Engine/EditorBlueprintResources/StandardMacros.IsValid` _murouest
    (:`Is Valid`
      (`StaticMeshComponent.SetStaticMesh` _murouest "/Game/MedievalDungeon/Meshes/Architecture/Dungeon/SM_Dungeon_Wall.SM_Dungeon_Wall")
      (`SceneComponent.K2_SetRelativeLocation` _murouest (600.0 0.0 0.0) false true))
    (:`Is Not Valid`
      (`/Engine/EditorBlueprintResources/StandardMacros.IsValid` _salleouest
        (:`Is Valid`
          (`self.AjoutMurEst` _salleouest))))))

(event `AjoutPorteOuest`
  (bind _murouest (`self.murOuest`))
  (bind _salleouest (`self.SalleOuest`))
  (`/Engine/EditorBlueprintResources/StandardMacros.IsValid` _murouest
    (:`Is Valid`
      (`StaticMeshComponent.SetStaticMesh` _murouest "/Game/MedievalDungeon/Meshes/Architecture/Dungeon/SM_DoorWay.SM_DoorWay")
      (`SceneComponent.K2_SetRelativeLocation` _murouest (300.0 0.0 0.0) false true))
    (:`Is Not Valid`
      (`/Engine/EditorBlueprintResources/StandardMacros.IsValid` _salleouest
        (:`Is Valid`
          (`self.AjoutPorteEst` _salleouest))
        (:`Is Not Valid`
          (`KismetSystemLibrary.PrintString` "Hello"))))))

(event `self.sol.OnClicked`
  (params (TouchedComponent :type "PrimitiveComponent Object Reference") (ButtonPressed :type "Key Structure")))

(event `SetSalleInfo`
  (params (Donnee :type String))
  (bind (_returnvalue_x _returnvalue_y _returnvalue_z) (`KismetMathLibrary.BreakVector` (`self.K2_GetActorLocation` self)))
  ;[1 1 1] Construction des murs et des portes
  (switch `string` Donnee
    (:`Default`
      (`KismetSystemLibrary.PrintString` Donnee))
    (:`(Nord)`
      (`self.AjoutPorteNord`)
      (switch `string` (`self.EvenementSalle`) :!label _label_2
        (:`Default`
          (if (> (`KismetMathLibrary.RandomIntegerInRange` 1 100) 50)
            (set `self.EvenementSalle` "Ennemi")
            (else
              (set `self.EvenementSalle` "Vide"))))
        (:`(Tresor)`
          (if (> (`KismetMathLibrary.RandomIntegerInRange` 1 100) 50)
            (set `self.EvenementSalle` "Piège")
            (else
              (set `self.EvenementSalle` "Trésor"))))
        (:`(Boss)`
          (set `self.EvenementSalle` "Boss"))
        (:`(Vision)`
          (set `self.EvenementSalle` "Vision"))
        (:`(J1)`
          (bind _returnvalue (`GameplayStatics.GetActorOfClass` "/Game/Blueprints/Actors/DonjonManager.DonjonManager_C"))
          (bind _player (`/Game/Blueprints/Actors/DonjonManager.Player` _returnvalue))
          (`self.K2_SetActorLocation` _player (`KismetMathLibrary.MakeVector` (+ _returnvalue_x 300.0) (+ _returnvalue_y 300.0) _returnvalue_z) false true)
          (`/Game/Blueprints/Pawns/Player.Lancement` _player)
          (set `/Game/Blueprints/Pawns/Player.SalleActuelle` self _player)
          (set `self.ConnueJ1` true)
          (`/Game/Blueprints/Pawns/Player.AffichageUIDeplacement` _player)
          (set `self.EvenementSalle` "Soin" :!label _label_3))
        (:`(J2)`
          (goto _label_3))
        (:`(Soin)`
          (set `self.EvenementSalle` "Soin"))))
    (:`(Sud)`
      (`self.AjoutPorteSud`)
      (goto _label_2))
    (:`(Est)`
      (`self.AjoutPorteEst`)
      (goto _label_2))
    (:`(Ouest)`
      (`self.AjoutPorteOuest`)
      (goto _label_2))
    (:`(Tresor)`
      (set `self.EvenementSalle` Donnee :!label _label_4)
      (goto _label_2))
    (:`(Boss)`
      (goto _label_4))
    (:`(Vision)`
      (goto _label_4))
    (:`(J1)`
      (goto _label_4))
    (:`(J2)`
      (goto _label_4))
    (:`(Nord,Sud)`
      (`self.AjoutPorteNord` :!label _label_5)
      (`self.AjoutPorteSud`)
      (goto _label_2))
    (:`(Sud,Nord)`
      (goto _label_5))
    (:`(Est,Nord)`
      (`self.AjoutPorteNord` :!label _label_6)
      (`self.AjoutPorteEst`)
      (goto _label_2))
    (:`(Nord,Est)`
      (goto _label_6))
    (:`(Est,Sud)`
      (`self.AjoutPorteSud` :!label _label_7)
      (`self.AjoutPorteEst`)
      (goto _label_2))
    (:`(Sud,Est)`
      (goto _label_7))
    (:`(Est,Ouest)`
      (`self.AjoutPorteEst` :!label _label_8)
      (`self.AjoutPorteOuest`)
      (goto _label_2))
    (:`(Ouest,Est)`
      (goto _label_8))
    (:`(Sud,Ouest)`
      (`self.AjoutPorteSud` :!label _label_9)
      (`self.AjoutPorteOuest`)
      (goto _label_2))
    (:`(Ouest,Sud)`
      (goto _label_9))
    (:`(Nord,Ouest)`
      (`self.AjoutPorteNord` :!label _label_10)
      (`self.AjoutPorteOuest`)
      (goto _label_2))
    (:`(Ouest,Nord)`
      (goto _label_10))
    (:`(Ouest,Est,Sud)`
      (`self.AjoutPorteOuest`)
      (`self.AjoutPorteEst`)
      (`self.AjoutPorteSud`)
      (goto _label_2))
    (:`(Sud,Ouest,Nord)`
      (`self.AjoutPorteSud`)
      (`self.AjoutPorteOuest`)
      (`self.AjoutPorteNord`)
      (goto _label_2))
    (:`(Nord,Est,Sud)`
      (`self.AjoutPorteNord` :!label _label_11)
      (`self.AjoutPorteEst`)
      (`self.AjoutPorteSud`)
      (goto _label_2))
    (:`(Sud,Est,Nord)`
      (goto _label_11))
    (:`(Soin)`
      (goto _label_4))))

(event `ViderLaSalle`
  (set `self.EvenementSalle` "Vide"))

(event `IconeSalle`
  (`self.ChangeIconeSalle`))

(fn `ChangeIconeSalle`
  (switch `string` (`self.EvenementSalle`)
    (:`Default`
      (`PaperSpriteComponent.SetSprite` (`self.PaperSpriteIcone`) "/Game/Pictures/icones/Inconnu_Sprite.Inconnu_Sprite" :!label _label))
    (:`Boss`
      (`PaperSpriteComponent.SetSprite` (`self.PaperSpriteIcone`) "/Game/Pictures/icones/Boss_Sprite.Boss_Sprite"))
    (:`Vision`
      (if (`self.ConnueJ1`)
        (`PaperSpriteComponent.SetSprite` (`self.PaperSpriteIcone`) "/Game/Pictures/icones/Vision_Sprite.Vision_Sprite")
        (else
          (goto _label))))
    (:`Trésor`
      (if (`self.ConnueJ1`)
        (`PaperSpriteComponent.SetSprite` (`self.PaperSpriteIcone`) "/Game/Pictures/icones/Tresor_Sprite.Tresor_Sprite")
        (else
          (goto _label))))
    (:`Piège`
      (if (`self.ConnueJ1`)
        (`PaperSpriteComponent.SetSprite` (`self.PaperSpriteIcone`) "/Game/Pictures/icones/Piege_Sprite.Piege_Sprite")
        (else
          (goto _label))))
    (:`Ennemi`
      (if (`self.ConnueJ1`)
        (`PaperSpriteComponent.SetSprite` (`self.PaperSpriteIcone`) "/Game/Pictures/icones/Ennemi_Sprite.Ennemi_Sprite")
        (else
          (goto _label))))
    (:`Vide`
      (if (`self.ConnueJ1`)
        (`PaperSpriteComponent.SetSprite` (`self.PaperSpriteIcone`) "/Game/Pictures/icones/Vide_Sprite.Vide_Sprite")
        (else
          (goto _label))))
    (:`Soin`
      (if (`self.ConnueJ1`)
        (`PaperSpriteComponent.SetSprite` (`self.PaperSpriteIcone`) "/Game/Pictures/icones/Soin_Sprite.Soin_Sprite")
        (else
          (goto _label))))))

(fn `Délétion murs et piliers`
  (if (not (or (`self.YBord`) (`self.XBord`)))
    (`ActorComponent.K2_DestroyComponent` (`self.pillierSudEst`)))
  ;[1 1 1] Gestion des cas particuliers des bords
  (if (not (`self.YBord`))
    (`ActorComponent.K2_DestroyComponent` (`self.murEst`)))
  (if (not (`self.XBord`))
    (`ActorComponent.K2_DestroyComponent` (`self.murSud`)))
  (if (not (and (`self.XBord`) (`self.-YBord`)))
    (`ActorComponent.K2_DestroyComponent` (`self.pillierSudOuest`)))
  (if (not (`self.-YBord`))
    (`ActorComponent.K2_DestroyComponent` (`self.pillierNordOuest`))))

(fn `MasqueMiniCarte`
  (bind _paperspritenord (`self.PaperSpriteNord`))
  (bind _paperspriteest (`self.PaperSpriteEst`))
  (bind _paperspritesud (`self.PaperSpriteSud`))
  (bind _paperspriteouest (`self.PaperSpriteOuest`))
  (if (and (`KismetSystemLibrary.IsValid` _paperspritenord) (`self.PorteNord`))
    (`ActorComponent.K2_DestroyComponent` _paperspritenord))
  (if (and (`KismetSystemLibrary.IsValid` _paperspriteest) (`self.PorteEst`))
    (`ActorComponent.K2_DestroyComponent` _paperspriteest))
  (if (and (`KismetSystemLibrary.IsValid` _paperspritesud) (`self.PorteSud`))
    (`ActorComponent.K2_DestroyComponent` _paperspritesud))
  (if (and (`KismetSystemLibrary.IsValid` _paperspriteouest) (`self.PorteOuest`))
    (`ActorComponent.K2_DestroyComponent` _paperspriteouest)))

(fn `PorteEst`
  (returns (Porte :type Boolean))
  (bind _murest (`self.murEst`))
  (`/Engine/EditorBlueprintResources/StandardMacros.IsValid` _murest
    (:`Is Valid`
      (return (== (`StaticMeshComponent.StaticMesh` _murest) "/Game/MedievalDungeon/Meshes/Architecture/Dungeon/SM_DoorWay.SM_DoorWay")))
    (:`Is Not Valid`
      (return (`self.PorteOuest` (`self.SalleEst`))))))

(fn `PorteNord`
  (returns (Porte :type Boolean))
  (bind _murnord (`self.murNord`))
  (`/Engine/EditorBlueprintResources/StandardMacros.IsValid` _murnord
    (:`Is Valid`
      (return (== (`StaticMeshComponent.StaticMesh` _murnord) "/Game/MedievalDungeon/Meshes/Architecture/Dungeon/SM_DoorWay.SM_DoorWay")))
    (:`Is Not Valid`
      (return (`self.PorteSud` (`self.SalleNord`))))))

(fn `PorteOuest`
  (returns (Porte :type Boolean))
  (bind _murouest (`self.murOuest`))
  (`/Engine/EditorBlueprintResources/StandardMacros.IsValid` _murouest
    (:`Is Valid`
      (return (== (`StaticMeshComponent.StaticMesh` _murouest) "/Game/MedievalDungeon/Meshes/Architecture/Dungeon/SM_DoorWay.SM_DoorWay")))
    (:`Is Not Valid`
      (return (`self.PorteEst` (`self.SalleOuest`))))))

(fn `PorteSud`
  (returns (Porte :type Boolean))
  (bind _mursud (`self.murSud`))
  (`/Engine/EditorBlueprintResources/StandardMacros.IsValid` _mursud
    (:`Is Valid`
      (return (== (`StaticMeshComponent.StaticMesh` _mursud) "/Game/MedievalDungeon/Meshes/Architecture/Dungeon/SM_DoorWay.SM_DoorWay")))
    (:`Is Not Valid`
      (return (`self.PorteNord` (`self.SalleSud`))))))

(fn `UserConstructionScript`)