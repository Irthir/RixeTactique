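; InstanceRixe is the Game Instance, holding host status (Hote) and a controller number (NControlleur) for the game session.
; SetHote stores the given host flag and sets the controller number to 1, while Reinitialiser clears both values.
; Network and travel error handlers only print the failure type as a debug string, with no recovery logic.
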(event `Reinitialiser`
  (set `self.bHote` false)
  (set `self.nControlleur` 0))

(event `SetHote`
  (params (bHote :type Boolean))
  (set `self.bHote` bHote)
  (set `self.nControlleur` 1))

(event `self.HandleNetworkError`
  (params (FailureType :type "ENetworkFailure Enum" :default "NetDriverAlreadyExists") (bIsServer :type Boolean))
  (`KismetSystemLibrary.PrintString` (`|GetEnumeratorNameAsString` FailureType)))

(event `self.HandleTravelError`
  (params (FailureType :type "ETravelFailure Enum" :default "NoLevel"))
  (`KismetSystemLibrary.PrintString` (`|GetEnumeratorNameAsString` FailureType)))