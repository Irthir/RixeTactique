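; Player pawn for a room-based dungeon crawler, steering a figurine with a smoothly following overhead camera and carrying a three-figurine team.
; BeginPlay starts DonjonManager and opens team selection, whose chosen data LancerJeu stores before showing movement UI.
; Directional actions move through doors, open the room's combat/event widget, reveal rooms (neighbours too with a scout effect) and count moves toward dungeon level.
; Potions heal the proportionally weakest teammate.
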(event `LancerJeu`
  (params (Figurine1 :type "Figurine Structure") (Figurine2 :type "Figurine Structure") (Figurine3 :type "Figurine Structure"))
  (`self.DataFigurine` Figurine1 Figurine2 Figurine3)
  (bind _returnvalue (`|CreateWidget` "/Game/Blueprints/Widgets/InterfaceDeplacement.InterfaceDeplacement_C"))
  (bind _output_get (set `self.InterfaceDeplacement` _returnvalue))
  (set `/Game/Blueprints/Widgets/InterfaceDeplacement.Joueur` self _output_get)
  (`UserWidget.AddToViewport` _output_get 0)
  (`self.Start`))

(event `SetDeplacementUI`
  (bind _returnvalue (`|CreateWidget` "/Game/Blueprints/Widgets/InterfaceDeplacement.InterfaceDeplacement_C"))
  (bind _output_get (set `self.InterfaceDeplacement` _returnvalue))
  (`UserWidget.AddToViewport` _output_get 0)
  (`self.AffichageUIDeplacement`))

(event `ChoixEquipe`
  (bind _returnvalue (`|CreateWidget` "/Game/Blueprints/Widgets/InterfaceChoixEquipe.InterfaceChoixEquipe_C" (`GameplayStatics.GetPlayerController` 0)))
  (`UserWidget.AddToViewport` _returnvalue 0))

(event `Connexion`
  (bind _returnvalue (`|CreateWidget` "/Game/Blueprints/Widgets/InterfaceConnexion.InterfaceConnexion_C"))
  (`UserWidget.AddToViewport` _returnvalue 0))

(event `DataFigurine`
  (params (Figurine1 :type "Figurine Structure") (Figurine2 :type "Figurine Structure") (Figurine3 :type "Figurine Structure"))
  (set `self.Figurine1` Figurine1)
  (set `self.Figurine2` Figurine2)
  (set `self.Figurine3` Figurine3))

(event `BeginPlay`
  (bind _returnvalue (`GameplayStatics.GetPlayerController` 0))
  (`WidgetBlueprintLibrary.SetInputMode_GameAndUIEx` (`GameplayStatics.GetPlayerController` 0) null)
  (`WidgetBlueprintLibrary.SetInputMode_GameAndUIEx` _returnvalue null)
  (set `PlayerController.bShowMouseCursor` true _returnvalue)
  (bind _returnvalue_2 (`GameplayStatics.GetActorOfClass` "/Game/Blueprints/Actors/DonjonManager.DonjonManager_C"))
  (set `self.DonjonManager` _returnvalue_2)
  (bind _asinstance_rixe (cast `/Game/Blueprints/GameInstance/InstanceRixe` (`GameplayStatics.GetGameInstance`)))
  (if (not (`/Game/Blueprints/GameInstance/InstanceRixe.bHote` _asinstance_rixe))
    (bind _outactors (`GameplayStatics.GetAllActorsOfClass` "Player_C"))
    (if (> (`KismetArrayLibrary.Array_Length` _outactors) 1)
      (`|SpawnActorFromClass` "/Game/Blueprints/Actors/NetWorkObject.NetWorkObject_C" (`KismetMathLibrary.MakeTransform` (0.0 0.0 0.0)) "AlwaysSpawn" "OverrideRootScale" null self)))
  (`/Game/Blueprints/Actors/DonjonManager.Lancement` (`self.DonjonManager`))
  (`self.ChoixEquipe`))

(event `self.ReceiveBeginPlay`
  (if (== (`GameplayStatics.GetPlayerPawn` 0) self)
    (`self.BeginPlay`)))

(event `Lancement`
  (bind _returnvalue (`|SpawnActorFromClass` "/Game/Blueprints/Actors/Figurine.Figurine_C" (`self.GetTransform` self) "AlwaysSpawn" "OverrideRootScale" self self))
  (set `self.Figurine` _returnvalue))

(event `Remove Event Salle`
  (`/Game/Blueprints/Actors/DonjonSalle.ViderLaSalle` (`self.SalleActuelle`)))

(event `self.ReceiveTick`
  (params (DeltaSeconds :type "Float (single-precision)"))
  (bind (_returnvalue_roll _returnvalue_pitch) (`KismetMathLibrary.BreakRotator` (`self.K2_GetActorRotation`)))
  (bind _returnvalue (+ DeltaSeconds 0.1))
  (bind (_returnvalue_x _returnvalue_y _returnvalue_z) (`KismetMathLibrary.BreakVector` (`self.K2_GetActorLocation` (`self.Figurine`))))
  (bind (_returnvalue_roll_2 _returnvalue_pitch_2) (`KismetMathLibrary.BreakRotator` (`KismetMathLibrary.FindLookAtRotation` (`self.K2_GetActorLocation`) (`self.K2_GetActorLocation` (`self.Figurine`)))))
  ;[1 1 1] Mouvement caméra
  (`/Engine/EditorBlueprintResources/StandardMacros.IsValid` (`self.Figurine`)
    (:`Is Valid`
      (`self.K2_SetActorRotation` (`KismetMathLibrary.MakeRotator` 0.0 (`KismetMathLibrary.Lerp` _returnvalue_pitch _returnvalue_pitch_2 _returnvalue)))
      (`self.K2_SetActorLocation` self (`KismetMathLibrary.VLerp` (`self.K2_GetActorLocation`) (`KismetMathLibrary.MakeVector` _returnvalue_x _returnvalue_y (+ _returnvalue_z 800.0)) _returnvalue) false false))))

(event `Key|A`
  (params (Key :type "Key Structure"))
  ;[1 1 1] Mouvement figurine
  (:`Pressed`
    (`self.ReinitDeplacement`)))

(event `ReinitDeplacement`
  ;[1 1 1] Mouvement figurine
  (set `self.DeplacementPossible` true)
  (`UserWidget.AddToViewport` (`self.InterfaceDeplacement`) 0))

(event `ActionNord`
  (bind _salleactuelle (`self.SalleActuelle`))
  (bind _salleactuelle_2 (`self.SalleActuelle`))
  (bind (_returnvalue_x _returnvalue_y _returnvalue_z) (`KismetMathLibrary.BreakVector` (`self.K2_GetActorLocation` (`self.SalleActuelle`))))
  ;[1 1 1] Mouvement figurine
  (if (`self.DeplacementPossible`) :!label _label
    (if (`/Game/Blueprints/Actors/DonjonSalle.PorteNord` _salleactuelle)
      (set `self.SalleActuelle` (`/Game/Blueprints/Actors/DonjonSalle.SalleNord` _salleactuelle))
      (set `/Game/Blueprints/Actors/Figurine.vTarget` (`KismetMathLibrary.MakeVector` (+ _returnvalue_x 300.0) (+ _returnvalue_y 300.0) _returnvalue_z) (`self.Figurine`) :!label _label_2)
      (set `self.DeplacementPossible` false)
      (`Widget.RemoveFromParent` (`self.InterfaceDeplacement`))
      (bind _asplayer_controller (cast `PlayerController` (`self.GetController`)))
      (bind _returnvalue (`|CreateWidget` "/Game/Blueprints/Widgets/InterfaceCombat.InterfaceCombat_C" _asplayer_controller))
      (`UserWidget.AddToViewport` _returnvalue 0)
      (`/Game/Blueprints/Widgets/InterfaceCombat.Evenement` _returnvalue self (`/Game/Blueprints/Actors/DonjonSalle.EvenementSalle` (`self.SalleActuelle`)))
      (`self.ConnaissanceSalle` _salleactuelle_2)
      (if (`self.bEclaireur`)
        (`self.ConnaissanceEnviron` _salleactuelle_2))
      (`self.AffichageUIDeplacement`)
      (`/Game/Blueprints/Actors/DonjonManager.TestVisibility` (`self.DonjonManager`))
      (`self.MouvementEffectue`))))

(event `InputAction|Nord`
  (params (Key :type "Key Structure"))
  ;[1 1 1] Mouvement figurine
  (:`Pressed`
    (goto _label)))

(event `ActionSud`
  (bind _salleactuelle (`self.SalleActuelle`))
  ;[1 1 1] Mouvement figurine
  (if (`self.DeplacementPossible`) :!label _label_3
    (if (`/Game/Blueprints/Actors/DonjonSalle.PorteSud` _salleactuelle)
      (set `self.SalleActuelle` (`/Game/Blueprints/Actors/DonjonSalle.SalleSud` _salleactuelle))
      (goto _label_2))))

(event `InputAction|Sud`
  (params (Key :type "Key Structure"))
  ;[1 1 1] Mouvement figurine
  (:`Pressed`
    (goto _label_3)))

(event `ActionEst`
  (bind _salleactuelle (`self.SalleActuelle`))
  ;[1 1 1] Mouvement figurine
  (if (`self.DeplacementPossible`) :!label _label_4
    (if (`/Game/Blueprints/Actors/DonjonSalle.PorteEst` _salleactuelle)
      (set `self.SalleActuelle` (`/Game/Blueprints/Actors/DonjonSalle.SalleEst` _salleactuelle))
      (goto _label_2))))

(event `InputAction|Est`
  (params (Key :type "Key Structure"))
  ;[1 1 1] Mouvement figurine
  (:`Pressed`
    (goto _label_4)))

(event `ActionOuest`
  (bind _salleactuelle (`self.SalleActuelle`))
  ;[1 1 1] Mouvement figurine
  (if (`self.DeplacementPossible`) :!label _label_5
    (if (`/Game/Blueprints/Actors/DonjonSalle.PorteOuest` _salleactuelle)
      (set `self.SalleActuelle` (`/Game/Blueprints/Actors/DonjonSalle.SalleOuest` _salleactuelle))
      (goto _label_2))))

(event `InputAction|Ouest`
  (params (Key :type "Key Structure"))
  ;[1 1 1] Mouvement figurine
  (:`Pressed`
    (goto _label_5)))

(event `InputAction|TPBoss`
  (params (Key :type "Key Structure"))
  ;[1 1 1] Mouvement figurine
)

(event `CarteVisible`
  ;[1 1 1] Mouvement figurine
  (bind _outactors (`GameplayStatics.GetAllActorsOfClass` "/Game/Blueprints/Actors/DonjonSalle.DonjonSalle_C" :!label _label_6))
  (for _array_element _outactors
    (bind _asdonjon_salle (cast `/Game/Blueprints/Actors/DonjonSalle` _array_element))
    (set `/Game/Blueprints/Actors/DonjonSalle.VueJ1` true _asdonjon_salle)
    (`/Game/Blueprints/Actors/DonjonSalle.TestVisibility` _asdonjon_salle))
  (bind _foundwidgets (`WidgetBlueprintLibrary.GetAllWidgetsOfClass` "/Game/Blueprints/Widgets/InterfaceDeplacement.InterfaceDeplacement_C" false))
  (for _array_element_2 _foundwidgets
    (`/Game/Blueprints/Widgets/InterfaceDeplacement.OpenMap` _array_element_2)))

(event `InputAction|Carte`
  (params (Key :type "Key Structure"))
  ;[1 1 1] Mouvement figurine
  (:`Pressed`
    (goto _label_6)))

(event `AffichageUIDeplacement`
  (bind _salleactuelle (`self.SalleActuelle`))
  (bind _interfacedeplacement (`self.InterfaceDeplacement`))
  ;[1 1 1] Mouvement figurine
  (`/Engine/EditorBlueprintResources/StandardMacros.IsValid` _interfacedeplacement
    (:`Is Valid`
      (`/Game/Blueprints/Widgets/InterfaceDeplacement.Affichage` _interfacedeplacement (`/Game/Blueprints/Actors/DonjonSalle.PorteNord` _salleactuelle) (`/Game/Blueprints/Actors/DonjonSalle.PorteEst` _salleactuelle) (`/Game/Blueprints/Actors/DonjonSalle.PorteSud` _salleactuelle) (`/Game/Blueprints/Actors/DonjonSalle.PorteOuest` _salleactuelle)))))

(event `Start`
  ;[1 1 1] Mouvement figurine
  (`self.AffichageUIDeplacement`))

(event `InputAction|Pause`
  (params (Key :type "Key Structure"))
  (bind _returnvalue (`GameplayStatics.GetPlayerController` 0))
  ;[1 1 1] Mouvement figurine
  (:`Pressed`
    (bind _returnvalue_2 (`|CreateWidget` "/Game/Blueprints/Widgets/InterfaceMenuPause.InterfaceMenuPause_C" _returnvalue))
    (`UserWidget.AddToViewport` _returnvalue_2 0)
    (`WidgetBlueprintLibrary.SetInputMode_UIOnlyEx` _returnvalue _returnvalue_2)
    (set `PlayerController.bShowMouseCursor` true _returnvalue)))

(fn `bEclaireur`
  (returns (bEclaireur :type Boolean))
  (bind (_figurine1_efigurine _figurine1_nvie _figurine1_nviemax _figurine1_nattaque _figurine1_nsoin _figurine1_eeffet) (break `Figurine` (`self.Figurine1`)))
  (bind (_figurine2_efigurine _figurine2_nvie _figurine2_nviemax _figurine2_nattaque _figurine2_nsoin _figurine2_eeffet) (break `Figurine` (`self.Figurine2`)))
  (bind (_figurine3_efigurine _figurine3_nvie _figurine3_nviemax _figurine3_nattaque _figurine3_nsoin _figurine3_eeffet) (break `Figurine` (`self.Figurine3`)))
  (return (or (`|EnumEquality` _figurine1_eeffet "VisionCase") (`|EnumEquality` _figurine2_eeffet "VisionCase") (`|EnumEquality` _figurine3_eeffet "VisionCase"))))

(fn `ConnaissanceEnviron`
  (params (Salle :type "/Game/Blueprints/Actors/DonjonSalle Object Reference"))
  (bind _sallenord (`/Game/Blueprints/Actors/DonjonSalle.SalleNord` Salle))
  (bind _sallesud (`/Game/Blueprints/Actors/DonjonSalle.SalleSud` Salle))
  (bind _salleouest (`/Game/Blueprints/Actors/DonjonSalle.SalleOuest` Salle))
  (bind _salleest (`/Game/Blueprints/Actors/DonjonSalle.SalleEst` Salle))
  (if (`/Game/Blueprints/Actors/DonjonSalle.PorteEst` Salle)
    (if true
      (set `/Game/Blueprints/Actors/DonjonSalle.ConnueJ1` true _salleest)
      (else
        (set `/Game/Blueprints/Actors/DonjonSalle.ConnueJ2` true _salleest))))
  (if (`/Game/Blueprints/Actors/DonjonSalle.PorteNord` Salle)
    (if true
      (set `/Game/Blueprints/Actors/DonjonSalle.ConnueJ1` true _sallenord)
      (else
        (set `/Game/Blueprints/Actors/DonjonSalle.ConnueJ2` true _sallenord))))
  (if (`/Game/Blueprints/Actors/DonjonSalle.PorteSud` Salle)
    (if true
      (set `/Game/Blueprints/Actors/DonjonSalle.ConnueJ1` true _sallesud)
      (else
        (set `/Game/Blueprints/Actors/DonjonSalle.ConnueJ2` true _sallesud))))
  (if (`/Game/Blueprints/Actors/DonjonSalle.PorteOuest` Salle)
    (if true
      (set `/Game/Blueprints/Actors/DonjonSalle.ConnueJ1` true _salleouest)
      (else
        (set `/Game/Blueprints/Actors/DonjonSalle.ConnueJ2` true _salleouest)))))

(fn `ConnaissanceSalle`
  (params (Salle :type "/Game/Blueprints/Actors/DonjonSalle Object Reference"))
  (if true
    (set `/Game/Blueprints/Actors/DonjonSalle.ConnueJ1` true Salle)
    (else
      (set `/Game/Blueprints/Actors/DonjonSalle.ConnueJ2` true Salle))))

(fn `getFigurinePVBas`
  (returns (Figurine :type "Figurine Structure"))
  (locals (`%Fig1` :type "Float (double-precision)") (`%Fig2` :type "Float (double-precision)") (`%Fig3` :type "Float (double-precision)"))
  (bind __fig2 (`local.%Fig2`))
  (bind (_figurine1_efigurine _figurine1_nvie _figurine1_nviemax) (break `Figurine` (`self.Figurine1`)))
  (bind (_figurine2_efigurine _figurine2_nvie _figurine2_nviemax) (break `Figurine` (`self.Figurine2`)))
  (bind (_figurine3_efigurine _figurine3_nvie _figurine3_nviemax) (break `Figurine` (`self.Figurine3`)))
  (bind __fig1 (`local.%Fig1`))
  (set `local.%Fig1` (/ (`KismetMathLibrary.Conv_IntToDouble` _figurine1_nvie) (`KismetMathLibrary.Conv_IntToDouble` _figurine1_nviemax)))
  (set `local.%Fig2` (/ (`KismetMathLibrary.Conv_IntToDouble` _figurine2_nvie) (`KismetMathLibrary.Conv_IntToDouble` _figurine2_nviemax)))
  (set `local.%Fig3` (/ (`KismetMathLibrary.Conv_IntToDouble` _figurine3_nvie) (`KismetMathLibrary.Conv_IntToDouble` _figurine3_nviemax)))
  (if (and (<= __fig1 (`local.%Fig2`)) (<= __fig1 (`local.%Fig3`)))
    (return (`self.Figurine1`))
    (elif (and (<= __fig2 (`local.%Fig1`)) (<= __fig2 (`local.%Fig3`)))
      (return (`self.Figurine2`))
      (else
        (return (`self.Figurine3`))))))

(fn `MouvementEffectue`
  (`/Engine/EditorBlueprintResources/StandardMacros.IncrementInt` (`self.NbMouvement`)
    (:`  `
      (if (> (+ (`self.NbMouvement`) 0) (* (`self.NiveauDonjon`) 10))
        (`/Engine/EditorBlueprintResources/StandardMacros.IncrementInt` (`self.NiveauDonjon`))))))

(fn `Potion`
  (bind (_figurine2_efigurine _figurine2_nvie _figurine2_nviemax) (break `Figurine` (`self.Figurine2`)))
  (bind (_figurine3_efigurine _figurine3_nvie _figurine3_nviemax) (break `Figurine` (`self.Figurine3`)))
  (bind _figurine1_efigurine (break `Figurine` (`self.Figurine1`)))
  (bind _figurine2_efigurine_2 (break `Figurine` (`self.Figurine2`)))
  (bind (_figurine1_efigurine_2 _figurine1_nvie _figurine1_nviemax) (break `Figurine` (`self.Figurine1`)))
  (if (and (> (`self.NbPotions`) 0) (or (< _figurine1_nvie _figurine1_nviemax) (< _figurine2_nvie _figurine2_nviemax) (< _figurine3_nvie _figurine3_nviemax)))
    (`/Engine/EditorBlueprintResources/StandardMacros.DecrementInt` (`self.NbPotions`)
      (:`  `
        (bind _figurine (`self.getFigurinePVBas`))
        (if (`|EnumEquality` (break `Figurine` _figurine) _figurine1_efigurine)
          (bind _figurinesoignee (`self.SoinPotion` (`self.Figurine1`)))
          (set `self.Figurine1` _figurinesoignee)
          (elif (`|EnumEquality` (break `Figurine` _figurine) _figurine2_efigurine_2)
            (bind _figurinesoignee_2 (`self.SoinPotion` (`self.Figurine2`)))
            (set `self.Figurine2` _figurinesoignee_2)
            (else
              (bind _figurinesoignee_3 (`self.SoinPotion` (`self.Figurine3`)))
              (set `self.Figurine3` _figurinesoignee_3))))))))

(fn `SoinPotion`
  (params (Figurine :type "Figurine Structure"))
  (returns (FigurineSoignee :type "Figurine Structure"))
  (return (make `Figurine` Figurine_eFigurine (`KismetMathLibrary.Clamp` (+ Figurine_nVie (/ Figurine_nVieMax 4)) 0 Figurine_nVieMax) Figurine_nVieMax Figurine_nAttaque Figurine_nSoin Figurine_eEffet Figurine_nNiveau Figurine_nExperience)))

(fn `UserConstructionScript`)